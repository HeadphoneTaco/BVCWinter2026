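; Side-scrolling moving platform Actor that slides its Cube to a target offset when triggered.
; A BPI_Interaction message or a Sphere overlap passes through a DoOnce gate to start the move.
; A FlipFlop alternates the destination between PlatformTarget and the relative origin, and Move Component To eases the Cube there over MoveDuration.
; Unless OneShot is set, the gate resets after the move so the platform can be triggered back.
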(event OnComponentBeginOverlap(Sphere)
  (params (OverlappedComponent :type Primitive%20Component%20Object%20Reference) (OtherActor :type Actor%20Object%20Reference) (OtherComp :type Primitive%20Component%20Object%20Reference) (OtherBodyIndex :type Integer) (bFromSweep :type Boolean) (SweepResult :type Hit%20Result%20Structure%20%28by%20ref%29))
  ;[0.15 0.15 0.15 0.5] As this Actor has the "BPI_Interaction" interface added in Class Settings, it can recieve an "Interaction" message as an event.
  ;
  ; On receiving the message, the Platform will activate it's movement behavior.
  (Utilities|FlowControl|DoOnce false ; We only want to activate the platform once
    (:Completed
      (CallFunction|MovetoTarget))))

(event Custom|Reset%20Interaction
  ;[0.15 0.15 0.15 0.5] As this Actor has the "BPI_Interaction" interface added in Class Settings, it can recieve an "Interaction" message as an event.
  ;
  ; On receiving the message, the Platform will activate it's movement behavior.
  (Utilities|FlowControl|DoOnce false) ; enters at Reset
)

(event Custom|Move%20to%20Target
  ;[0.15 0.15 0.15 0.5] As this Actor has the "BPI_Interaction" interface added in Class Settings, it can recieve an "Interaction" message as an event.
  ;
  ; On receiving the message, the Platform will activate it's movement behavior.
  (bind _isa (Utilities|FlowControl|FlipFlop)
    (:A
      _)
    (:B
      _))
  (Components|MoveComponentTo (Variables|Default|GetCube) (Math|Vector|SelectVector (Variables|MovingPlatform|GetPlatform%20Target) "0, 0, 0" _isa) "0, 0, 0" true true (Variables|MovingPlatform|GetMove%20Duration) false)
  (if (not (Variables|MovingPlatform|GetOne%20Shot))
    (CallFunction|ResetInteraction)))

(event EventInteraction
  (params (Interactor :type Actor%20Object%20Reference))
  ;[0.15 0.15 0.15 0.5] As this Actor has the "BPI_Interaction" interface added in Class Settings, it can recieve an "Interaction" message as an event.
  ;
  ; On receiving the message, the Platform will activate it's movement behavior.
  (Utilities|FlowControl|DoOnce false ; We only want to activate the platform once
    (:Completed
      (CallFunction|MovetoTarget))))

(fn ConstructionScript)