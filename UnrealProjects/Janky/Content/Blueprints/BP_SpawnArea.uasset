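; BP_SpawnArea is a triggered spawn zone that scatters BP_Battery pickups the first time BP_Player enters its TriggerBox.
; A DoOnce gate runs a loop up to MaxNumberofSpawns, placing each battery at a random point inside the SpawnExtent box.
; Spawning adjusts for collisions or skips blocked placements, and each battery's lifetime timer starts with TimeToCollect.
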(event OnComponentBeginOverlap(TriggerBox)
  (params (OverlappedComponent :type Primitive%20Component%20Object%20Reference) (OtherActor :type Actor%20Object%20Reference) (OtherComp :type Primitive%20Component%20Object%20Reference) (OtherBodyIndex :type Integer) (bFromSweep :type Boolean) (SweepResult :type Hit%20Result%20Structure%20%28by%20ref%29))
  (Utilities|Casting|CastToBP_Player OtherActor)
  (Utilities|FlowControl|DoOnce false
    (:Completed
      (for _index (range 0 (Variables|SpawnDetails|GetMaxNumberofSpawns))
        (bind _returnvalue (Game|SpawnActorfromClass "/Game/Blueprints/BP_Battery.BP_Battery_C" (Math|Transform|MakeTransform (CallFunction|GetRandomLocationinSpawn) "0, 0, 0" "1.000000,1.000000,1.000000") "AdjustIfPossibleButDontSpawnIfColliding" "MultiplyWithRoot" 0 0))
        (Default|StartLifetimeTimer _returnvalue (Variables|SpawnDetails|GetTimeToCollect))))))

(fn ConstructionScript)

(fn GetRandomLocationinSpawn
  (bind _spawnextent (Variables|Default|GetSpawnExtent))
  (return (Math|Random|RandomPointinBoundingBox (Transformation|GetWorldLocation _spawnextent) (Variables|/Script/Engine.BoxComponent|GetBoxExtent _spawnextent))))