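; BP_Door is a door that opens through a timeline once enough pressure switches are active, and doubles as a checkpoint.
; Switch events adjust a counter; reaching the required count saves the door's location to BP_Player and BP_MyGameInstance.
; A DoorSaved flag limits both the opened-door tally and the timeline's Play to the first activation.
; Dropping below the required count reverses the timeline.
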(event Custom|SwitchActivated
  (Math|Integer|IncrementInt (Variables|Default|GetPressureSwitchesActive)
    (:%20%20
      (if (== (Variables|Default|GetPressureSwitchesActive) (Variables|Default|GetPressureSwitchesNeeded))
        (bind _asbp_player (Utilities|Casting|CastToBP_Player (Game|GetPlayerCharacter 0)))
        (Variables|/Game/Player/BP_Player.BP_Player_C|SetCheckpointLocation _asbp_player (Transformation|GetActorLocation))
        (bind _asbp_my_game_instance (Utilities|Casting|CastToBP_MyGameInstance (Game|GetGameInstance)))
        (Default|SaveCheckpoint _asbp_my_game_instance (Transformation|GetActorLocation))
        (if (not (Variables|Default|GetbDoorSaved))
          (Default|IncrementDoorsOpened _asbp_my_game_instance)
          (Variables|Default|SetbDoorSaved true)
          (bind _doorposition (Timeline|DoorActivation Play)
            (:Update
              (Transformation|SetRelativeLocation (Variables|Default|GetDoor) (Math|Vector|MakeVector 0.0 0.0 _doorposition) false false))))))))

(event Custom|SwitchDeactivated
  (Math|Integer|DecrementInt (Variables|Default|GetPressureSwitchesActive)
    (:%20%20
      (if (< (Variables|Default|GetPressureSwitchesActive) (Variables|Default|GetPressureSwitchesNeeded))
        (bind _doorposition (Timeline|DoorActivation Reverse)
          (:Update
            (Transformation|SetRelativeLocation (Variables|Default|GetDoor) (Math|Vector|MakeVector 0.0 0.0 _doorposition) false false)))))))

(fn ConstructionScript)