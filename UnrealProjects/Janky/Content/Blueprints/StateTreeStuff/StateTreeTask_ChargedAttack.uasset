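; StateTree task that makes an enemy character perform a charged attack and holds the state until the attack ends.
; On entering the state it binds to the character's Attack Completed event and triggers the AI charged attack, finishing successfully when that event fires.
; On exiting the state it unbinds the event, and both hooks act only on transitions whose change type is Changed.
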(event Custom|Attack%20Completed
  ;[0.15 0.15 0.15 0.5] Finish this task when the enemy is done attacking.
  (StateTree|FinishTask true))

(event EventLatentEnterState
  (params (Transition :type State%20Tree%20Transition%20Result%20Structure%20%28by%20ref%29))
  (bind _character (Variables|Context|GetCharacter))
  ;[0.15 0.15 0.15 0.5] Set up the attack when entering into this state
  ;;[0.15 0.15 0.15 0.5] We only care about transitions that enter into this state.
  (if (Utilities|Enum|Equal(Enum) (.changetype Transition) "Changed")
    ;;[0.15 0.15 0.15 0.5] Subscribe to the Attack Completed event on the enemy.
    (EventDispatchers|BindEventtoOnAttackCompleted _character (delegate Custom|Attack%20Completed))
    ;;[0.15 0.15 0.15 0.5] Tell the enemy to do a charged attack.
    (Default|DoAIChargedAttack _character)))

(event EventExitState
  (params (Transition :type State%20Tree%20Transition%20Result%20Structure%20%28by%20ref%29))
  ;[0.15 0.15 0.15 0.5] Clean up when exiting this state
  ;;[0.15 0.15 0.15 0.5] We only care about transitions that exit out of this state.
  (if (Utilities|Enum|Equal(Enum) (.changetype Transition) "Changed")
    ;;[0.15 0.15 0.15 0.5] Unsubscribe from the Attack Completed event.
    (EventDispatchers|UnbindEventfromOnAttackCompleted (Variables|Context|GetCharacter) (delegate Custom|Attack%20Completed))))