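; StateTree task that holds a state until its Character lands.
; On a changed-state enter it binds to the Character's Landed delegate and finishes successfully when that fires.
; On a changed-state exit it unbinds the delegate, ignoring transitions that merely sustain the state.
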(event Custom|Landed
  (params (Hit :type Hit%20Result%20Structure%20%28by%20ref%29))
  ;[0.15 0.15 0.15 0.5] Finish the task as soon as the character lands
  (StateTree|FinishTask true))

(event EventLatentEnterState
  (params (Transition :type State%20Tree%20Transition%20Result%20Structure%20%28by%20ref%29))
  ;[0.15 0.15 0.15 0.5] Listen for landing events on State enter, and wait until the character lands.
  ;;[0.15 0.15 0.15 0.5] We only care about transitions that enter into this state
  (if (Utilities|Enum|Equal(Enum) (.changetype Transition) "Changed")
    ;;[0.15 0.15 0.15 0.5] Subscribe to landing events on the character
    (EventDispatchers|BindEventtoLandedDelegate (Variables|Context|GetCharacter) (delegate Custom|Landed))))

(event EventExitState
  (params (Transition :type State%20Tree%20Transition%20Result%20Structure%20%28by%20ref%29))
  ;[0.15 0.15 0.15 0.5] Clean up when this State exits.
  ;;[0.15 0.15 0.15 0.5] We only care about transitions that exit from this state
  (if (Utilities|Enum|Equal(Enum) (.changetype Transition) "Changed")
    ;;[0.15 0.15 0.15 0.5] Unsubscribe from landing events
    (EventDispatchers|UnbindEventfromLandedDelegate (Variables|Context|GetCharacter) (delegate Custom|Landed))))