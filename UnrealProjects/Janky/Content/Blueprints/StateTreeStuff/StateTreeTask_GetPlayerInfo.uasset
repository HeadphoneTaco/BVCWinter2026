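; StateTree task that tracks the player pawn as an attack target.
; On each latent tick it takes the pawn of player index 0 and, if valid, stores its current location as the last known target location.
; It also saves the straight-line distance from the AttackSource actor to that pawn.
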(event EventLatentTick
  (params (DeltaTime :type Float%20%28single-precision%29))
  ;[0.15 0.15 0.15 0.5] Set the Pawn to try and attack
  (Variables|Outputs|SetTarget%20Player%20Character (Game|Player|GetPlayerPawn 0))
  (Utilities|IsValid (Variables|Outputs|GetTarget%20Player%20Character)
    (:Is%20Valid
      ;[0.15 0.15 0.15 0.5] Set the last known location of the target.
      (Variables|Outputs|SetTarget%20Player%20Location (Transformation|GetActorLocation (Variables|Outputs|GetTarget%20Player%20Character)))
      ;[0.15 0.15 0.15 0.5] Calculate and save the linear distance to the target.
      (Variables|Outputs|SetDistance%20to%20Target (Math|Vector|VectorLength (- (Transformation|GetActorLocation (Variables|Outputs|GetTarget%20Player%20Character)) (Transformation|GetActorLocation (Variables|Context|GetAttack%20Source))))))))