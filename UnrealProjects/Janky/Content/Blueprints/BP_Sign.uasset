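; BP_Sign is a maze game sign actor that shows its message when the player enters its trigger sphere.
; The overlap stores SignMessage on BP_Player and passes it to BP_MazeGameMode for display.
; The construction script creates a dynamic material, setting "CoinColor" rather than the "SignColor" parameter animated at runtime.
; From BeginPlay, a timeline blends that material between two colors and destroys the actor if it finishes.
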(event OnComponentBeginOverlap(TriggerSphere)
  (params (OverlappedComponent :type Primitive%20Component%20Object%20Reference) (OtherActor :type Actor%20Object%20Reference) (OtherComp :type Primitive%20Component%20Object%20Reference) (OtherBodyIndex :type Integer) (bFromSweep :type Boolean) (SweepResult :type Hit%20Result%20Structure%20%28by%20ref%29))
  (bind _asbp_maze_player (Utilities|Casting|CastToBP_Player OtherActor))
  (Variables|/Game/Player/BP_Player.BP_Player_C|SetMostRecentDebugMessage _asbp_maze_player (Variables|SignDetails|GetSignMessage))
  (bind _asbp_maze_game_mode (Utilities|Casting|CastToBP_MazeGameMode (Game|GetGameMode)))
  (Default|DisplaySignMessage _asbp_maze_game_mode (Variables|SignDetails|GetSignMessage)))

(event EventBeginPlay
  (bind _colortrack (Timeline|ColorTimeline Play)
    (:Update
      (Rendering|Material|SetVectorParameterValue (Variables|SignDetails|GetSignMaterial) "SignColor" (Math|Color|Lerp(LinearColor) (Variables|SignDetails|GetSignColorA) (Variables|SignDetails|GetSignColorB) _colortrack) :!class /Script/Engine.MaterialInstanceDynamic))
    (:Finished
      (Actor|DestroyActor))))

(fn ConstructionScript
  (bind _returnvalue (Rendering|Material|CreateDynamicMaterialInstance (Variables|Default|GetSignMesh) 0 0 "None" :!class /Script/Engine.PrimitiveComponent))
  (bind _output_get (Variables|SignDetails|SetSignMaterial _returnvalue))
  (Rendering|Material|SetVectorParameterValue _output_get "CoinColor" (Variables|SignDetails|GetSignColor) :!class /Script/Engine.MaterialInstanceDynamic))