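; Game instance that manages persistent progress (checkpoint, keys, opened doors) through a BP_MySaveData save object.
; On Init it loads the default slot or creates a new save, restoring checkpoint and doors but only printing the saved key total.
; Checkpoint and key events update runtime values and write the slot immediately.
; SaveCheckpoint assigns the saved location to itself, so the new location never reaches the save.
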(event Custom|IncrementKeyAmount
  (bind _savegamedata (Variables|Default|GetSaveGameData))
  (bind _result (Math|Integer|IncrementInt (Variables|Default|GetTotalKeysCollected))
    (:%20%20
      (Development|PrintString (Utilities|String|ToString(Integer) _result))
      (Math|Integer|IncrementInt (Variables|/Game/Blueprints/BP_MySaveData.BP_MySaveData_C|GetSavedTotalKeysCollected _savegamedata)
        (:%20%20
          (SaveGame|SaveGametoSlot _savegamedata (Variables|Default|GetDefaultSaveSlot)))))))

(event Custom|SaveCheckpoint
  (params (Location :type Vector))
  (bind _savegamedata (Variables|Default|GetSaveGameData))
  (Development|PrintString "SaveCheckpoint called" true true "(R=0.000000,G=0.660000,B=1.000000,A=1.000000)" 2.0 "SaveCheckpoint")
  (Variables|Default|SetCheckpointLocation Location)
  (Variables|/Game/Blueprints/BP_MySaveData.BP_MySaveData_C|SetSavedCheckpointLocation _savegamedata (Variables|/Game/Blueprints/BP_MySaveData.BP_MySaveData_C|GetSavedCheckpointLocation _savegamedata))
  (SaveGame|SaveGametoSlot _savegamedata (Variables|Default|GetDefaultSaveSlot)))

(event EventInit
  (bind _returnvalue (SaveGame|DoesSaveGameExist (Variables|Default|GetDefaultSaveSlot)))
  (if _returnvalue
    (CallFunction|LoadExistingSave)
    (else
      (CallFunction|CreateNewSave))))

(fn CreateNewSave
  (bind _returnvalue (SaveGame|CreateSaveGameObject "/Game/Blueprints/BP_MySaveData.BP_MySaveData_C"))
  (bind _output_get (Variables|Default|SetSaveGameData _returnvalue))
  (SaveGame|SaveGametoSlot _output_get (Variables|Default|GetDefaultSaveSlot)))

(fn LoadExistingSave
  (bind _returnvalue (SaveGame|LoadGamefromSlot (Variables|Default|GetDefaultSaveSlot)))
  (bind _asbp_my_save_data (Utilities|Casting|CastToBP_MySaveData _returnvalue))
  (Variables|Default|SetSaveGameData _asbp_my_save_data)
  (Variables|Default|SetCheckpointLocation (Variables|/Game/Blueprints/BP_MySaveData.BP_MySaveData_C|GetSavedCheckpointLocation _asbp_my_save_data))
  (Variables|Default|SetDoorsOpened (Variables|/Game/Blueprints/BP_MySaveData.BP_MySaveData_C|GetSavedDoorsOpened _asbp_my_save_data))
  (Development|PrintString (Utilities|String|Append "Game Loaded. Total Keys:" (Utilities|String|ToString(Integer) (Variables|/Game/Blueprints/BP_MySaveData.BP_MySaveData_C|GetSavedTotalKeysCollected _asbp_my_save_data)))))