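; BP_Ghost is a maze enemy that chases the player pawn, cached as its target on BeginPlay.
; Each Tick it faces the target and moves forward unswept, without navigation, while beyond a distance threshold.
; TakeDamage lowers health and, at the death threshold, reports its location to BP_MazeGameMode before destroying itself.
; Overlap calls DealDamage, which is still an empty stub, and debug prints trace health, distance and rotation.
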(event EventBeginPlay
  (bind _asbp_player (Utilities|Casting|CastToBP_Player (Game|Player|GetPlayerPawn 0)))
  (Variables|Prey|SetTargetRef _asbp_player)
  (Variables|Pred|SetEntitySpawnLocation (Variables|Pred|GetEntitySpawnLocation)))

(event Collision|EventActorBeginOverlap
  (params (OtherActor :type Actor%20Object%20Reference))
  (CallFunction|DealDamage))

(event EventTick
  (params (DeltaSeconds :type Float%20%28single-precision%29))
  (CallFunction|ChasetheTarget))

(fn ConstructionScript)

(fn DealDamage)

(fn TakeDamage
  (params (Damage :type Float%20%28double-precision%29))
  (bind _output_get (Variables|Pred|SetEntityHealth (- (Variables|Pred|GetEntityHealth) Damage)))
  (Development|PrintString (Utilities|String|Append "Entity Health : " (Utilities|String|ToString(Float) _output_get)) true true "(R=0.000000,G=1.000000,B=0.046954,A=1.000000)" 2e+01 "EntityHealth")
  (if (<= (Variables|Pred|GetEntityHealth) (Variables|Pred|GetDeathThreshold))
    (bind _output_get_2 (LocalVariables|SetMyLocation (Transformation|GetActorLocation)))
    (Development|PrintString (Utilities|String|Append "Entity Location : " (Utilities|String|ToString(Vector) _output_get_2)) true true "(R=1.000000,G=0.978739,B=0.000000,A=1.000000)" 2e+01 "EntityLocation")
    (bind _asbp_maze_game_mode (Utilities|Casting|CastToBP_MazeGameMode (Game|GetGameMode)))
    (Default|OnEntityDeath _asbp_maze_game_mode (LocalVariables|GetMyLocation))
    (Actor|DestroyActor)))

(fn ChasetheTarget
  (Variables|Pred|SetEntityLocation (Transformation|GetActorLocation))
  (Variables|Prey|SetTargetLocation (Transformation|GetActorLocation (Variables|Prey|GetTargetRef)))
  (Variables|Prey|SetDistanceToTarget (Math|Vector|Distance(Vector) (Variables|Pred|GetEntityLocation) (Variables|Prey|GetTargetLocation)))
  (Development|PrintString (Utilities|String|Append "Distance to Target : " (Utilities|String|ToString(Float) (Variables|Prey|GetDistanceToTarget))) true true "(R=1.000000,G=0.296035,B=0.000000,A=1.000000)" 2e+01 "TargetDistance")
  (if (< (Variables|Prey|GetDistanceThreshold) (Variables|Prey|GetDistanceToTarget))
    (Development|PrintString (Utilities|String|Append "Rotation Values : " (Utilities|String|ToString(Rotator) (Math|Rotator|FindLookatRotation (Variables|Pred|GetEntityLocation) (Variables|Prey|GetTargetLocation)))) true true "(R=0.389481,G=0.000000,B=1.000000,A=1.000000)" 2e+01 "ChaseRotation")
    (Transformation|SetActorRotation (Math|Rotator|FindLookatRotation (Variables|Pred|GetEntityLocation) (Variables|Prey|GetTargetLocation)))
    (Transformation|AddActorWorldOffset (* (Transformation|GetActorForwardVector) (* (Utilities|Time|GetWorldDeltaSeconds) (Variables|Pred|GetMoveSpeed))))))